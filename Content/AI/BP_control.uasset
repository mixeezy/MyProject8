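; BP_control is an AI controller for an NPC that tracks the player through AI perception.
; On BeginPlay it runs the BT_npc behavior tree and sets the IsForward blackboard flag to true.
; Perception updates for player character 0 write that actor to the "player" blackboard key when sensed and clear the key when sensing fails, ignoring all other actors.
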(event OnTargetPerceptionUpdated(AIPerception)
  (params (Actor :type Actor%20Object%20Reference) (Stimulus :type AI%20Stimulus%20Structure))
  (if (== Actor (Game|GetPlayerCharacter 0))
    (if (.bSuccessfullySensed (Utilities|Struct|BreakAIStimulus Stimulus))
      (AI|Components|Blackboard|SetValueasObject (Variables|Default|GetBlackboard) (Utilities|String|StringToName "player") Actor)
      (else
        (AI|Components|Blackboard|ClearValue (Variables|Default|GetBlackboard) (Utilities|String|StringToName "player"))))))

(event EventBeginPlay
  (AI|RunBehaviorTree "/Game/AI/BT_npc.BT_npc")
  (AI|Components|Blackboard|SetValueasBool (Variables|Default|GetBlackboard) (Utilities|Name|MakeLiteralName "IsForward") true))

(fn ConstructionScript)