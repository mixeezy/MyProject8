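; BP_NPC is an NPC that damages the third-person player character while it stays inside the NPC's Sphere trigger.
; Sphere overlap events store the character and set an Overlap flag, and Tick calls the character's TakeDamage every frame while it is set, with no delta-time scaling.
; BeginPlay caches the world locations of the Spline's points in an array, which this graph never reads.
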(event OnComponentBeginOverlap(Sphere)
  (params (OverlappedComponent :type Primitive%20Component%20Object%20Reference) (OtherActor :type Actor%20Object%20Reference) (OtherComp :type Primitive%20Component%20Object%20Reference) (OtherBodyIndex :type Integer) (bFromSweep :type Boolean) (SweepResult :type Hit%20Result%20Structure%20%28by%20ref%29))
  (bind _asbp_third_person_character (Utilities|Casting|CastToBP_ThirdPersonCharacter OtherActor))
  (Variables|Default|SetAs%20BP%20Third%20Person%20Character _asbp_third_person_character)
  (Variables|Default|Setoverlap true))

(event OnComponentEndOverlap(Sphere)
  (params (OverlappedComponent :type Primitive%20Component%20Object%20Reference) (OtherActor :type Actor%20Object%20Reference) (OtherComp :type Primitive%20Component%20Object%20Reference) (OtherBodyIndex :type Integer))
  (if (== OtherActor (Variables|Default|GetAs%20BP%20Third%20Person%20Character))
    (Variables|Default|SetAs%20BP%20Third%20Person%20Character 0)
    (Variables|Default|Setoverlap false)))

(event EventTick
  (params (DeltaSeconds :type Float%20%28single-precision%29))
  (if (Variables|Default|Getoverlap)
    (Default|TakeDamage (Variables|Default|GetAs%20BP%20Third%20Person%20Character) (Variables|Default|Getdamage))))

(event EventBeginPlay
  (Utilities|Array|Clear (Variables|Default|GetSplnePointLocations))
  (for _index (range 0 (- (Spline|GetNumberOfSplinePoints (Variables|Default|GetSpline)) 1))
    (Utilities|Array|Add (Variables|Default|GetSplnePointLocations) (Spline|GetLocationatSplinePoint (Variables|Default|GetSpline) _index "World"))))

(fn ConstructionScript)