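; BP_key is an interactable key pickup that grants keys to the player.
; On Interact it adds five to the Keys count on the third-person character.
; It then refreshes the key counter widget inside the game mode's HealthBar UI and destroys itself.
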(event EventInteract
  (bind _asbp_third_person_character (Utilities|Casting|CastToBP_ThirdPersonCharacter (Game|GetPlayerCharacter 0)))
  (bind _output_get (Variables|/Game/ThirdPerson/Blueprints/BP_ThirdPersonCharacter.BP_ThirdPersonCharacter_C|Setkeys _asbp_third_person_character (+ (Variables|/Game/ThirdPerson/Blueprints/BP_ThirdPersonCharacter.BP_ThirdPersonCharacter_C|Getkeys _asbp_third_person_character) 5)))
  (bind _asbp_third_person_game_mode (Utilities|Casting|CastToBP_ThirdPersonGameMode (Game|GetGameMode)))
  (Default|UpdateKeys (Variables|/Game/IntractiveObject/UI_health.UI_health_C|GetUI_keys (Variables|/Game/ThirdPerson/Blueprints/BP_ThirdPersonGameMode.BP_ThirdPersonGameMode_C|Gethealth%20bar _asbp_third_person_game_mode)) _output_get)
  (Actor|DestroyActor))

(fn ConstructionScript
  (|CallParentFunction))