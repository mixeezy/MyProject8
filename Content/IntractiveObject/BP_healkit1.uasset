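; BP_healkit1 is an interactable pickup actor, named as a heal kit, that is consumed on use.
; Its Interact event casts player 0 to BP_ThirdPersonCharacter, passes its Damage variable to that character's TakeDamage, then destroys itself.
; Any healing depends on that value and function, as no separate heal call exists.
; A disconnected branch that would update the game mode's health bar never runs.
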(event EventInteract
  (bind _asbp_third_person_character (Utilities|Casting|CastToBP_ThirdPersonCharacter (Game|GetPlayerCharacter 0)))
  (Default|TakeDamage _asbp_third_person_character (Variables|Default|Getdamage))
  (Actor|DestroyActor))

(fn ConstructionScript
  (|CallParentFunction))