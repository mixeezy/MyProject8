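; BP_lock is an interactive lock actor that takes one of the player's keys and destroys itself.
; On Interact it reads the Keys count on BP_ThirdPersonCharacter and proceeds only when that count is five or fewer, with no check for zero.
; It then decrements the count, pushes it to the Keys object on BP_ThirdPersonGameMode through UpdateKeys, and removes the lock.
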(event EventInteract
  (bind _asbp_third_person_character (Utilities|Casting|CastToBP_ThirdPersonCharacter (Game|GetPlayerCharacter 0)))
  (if (<= (Variables|/Game/ThirdPerson/Blueprints/BP_ThirdPersonCharacter.BP_ThirdPersonCharacter_C|Getkeys _asbp_third_person_character) 5)
    (bind _output_get (Variables|/Game/ThirdPerson/Blueprints/BP_ThirdPersonCharacter.BP_ThirdPersonCharacter_C|Setkeys _asbp_third_person_character (- (Variables|/Game/ThirdPerson/Blueprints/BP_ThirdPersonCharacter.BP_ThirdPersonCharacter_C|Getkeys _asbp_third_person_character) 1)))
    (bind _asbp_third_person_game_mode (Utilities|Casting|CastToBP_ThirdPersonGameMode (Game|GetGameMode)))
    (Default|UpdateKeys (Variables|/Game/ThirdPerson/Blueprints/BP_ThirdPersonGameMode.BP_ThirdPersonGameMode_C|Getkeys _asbp_third_person_game_mode) _output_get)
    (Actor|DestroyActor)))

(fn ConstructionScript
  (|CallParentFunction))